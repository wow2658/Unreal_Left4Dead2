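; Elevator model actor with door open and close events and a proximity text prompt.
; The door events set IsOpen and play or reverse a Timeline, but its update drives nothing and their bindings never run.
; The box overlap toggles the text and input on player controller 0.
; Pressing or releasing C snaps two inner frame meshes to fixed positions, one in world space, one relative.
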(event `OpenDoor`
  (set `self.IsOpen` true)
  ;[1 1 1] 앞문
  (`Timeline|Timeline` :!label _label
    (:`Update`
      (`|ExecutionSequence`))))

(event `self.Box.OnComponentBeginOverlap`
  (params (OverlappedComponent :type "PrimitiveComponent Object Reference") (OtherActor :type "Actor Object Reference") (OtherComp :type "PrimitiveComponent Object Reference") (OtherBodyIndex :type Integer) (bFromSweep :type Boolean) (SweepResult :type "HitResult Structure (by ref)"))
  (`SceneComponent.SetVisibility` (`self.TextRender`) true false)
  (`self.EnableInput` (`GameplayStatics.GetPlayerController` 0) null))

(event `CloseDoor`
  (set `self.IsOpen` false)
  (goto _label :!via `Reverse`))

(event `self.Box.OnComponentEndOverlap`
  (params (OverlappedComponent :type "PrimitiveComponent Object Reference") (OtherActor :type "Actor Object Reference") (OtherComp :type "PrimitiveComponent Object Reference") (OtherBodyIndex :type Integer))
  (`SceneComponent.SetVisibility` (`self.TextRender`) false false)
  (`self.DisableInput` (`GameplayStatics.GetPlayerController` 0) null))

(event `Key|E`
  (params (Key :type "Key Structure")))

(event `Key|C` :paused true
  (params (Key :type "Key Structure"))
  (:`Pressed`
    (`|ExecutionSequence` :!label _label_2
      (:`then_0`
        (`SceneComponent.K2_SetWorldLocation` (`self.SM_Elevator_InnerFrame_11`) (-1210.0 1370.0 0.0) false false))
      (:`then_1`
        (`SceneComponent.K2_SetRelativeLocation` (`self.SM_Elevator_InnerFrame_12`) (70.0 0.0 0.0) false false))))
  (:`Released`
    (goto _label_2)))

(event `self.ReceiveTick`
  (params (DeltaSeconds :type "Float (single-precision)")))

(fn `UserConstructionScript`)