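; BP_Gas is an interactable gas pickup that BP_Hank can carry.
; On Interacted, while IsActive, it casts the interactor to BP_Hank and chains through Gas to GasM.
; If Hank's GAS reference is empty, GasM attaches the actor to him, offsets and rotates the mesh, disables its physics and stores itself in that reference, limiting Hank to one at a time.
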(event `/Game/Dev/LGT/Interacted.Interacted`
  (params (Interactor :type "Pawn Object Reference"))
  (if true
    (if (`self.bIsActive`)
      (bind _asbp_hank (cast `/Game/Dev/LGT/Hank_BP/BP_Hank` Interactor))
      (`self.Gas`))))

(event `Gas`
  (`self.GasM`))

(event `GasM`
  (bind _meshcomp (`self.meshComp`))
  (`/Engine/EditorBlueprintResources/StandardMacros.IsValid` (`/Game/Dev/LGT/Hank_BP/BP_Hank.GAS` (stale `/Game/Dev/LGT/Interacted.Interacted` _asbp_hank))
    (:`Is Not Valid`
      (`self.K2_AttachToActor` (stale `/Game/Dev/LGT/Interacted.Interacted` _asbp_hank) "None" "KeepRelative" "KeepRelative" "KeepRelative")
      (`SceneComponent.K2_SetRelativeLocation` _meshcomp (50.0 0.0 40.0) false false)
      (`SceneComponent.K2_SetRelativeRotation` _meshcomp (struct :`Yaw` 90.0) false false)
      (`PrimitiveComponent.SetSimulatePhysics` _meshcomp false)
      (set `self.bIsActive` true)
      (set `/Game/Dev/LGT/Hank_BP/BP_Hank.GAS` self (stale `/Game/Dev/LGT/Interacted.Interacted` _asbp_hank)))))

(fn `UserConstructionScript`)