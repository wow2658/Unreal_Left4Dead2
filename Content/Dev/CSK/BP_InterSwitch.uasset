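; BP_InterSwitch is a one-shot overlap switch that activates the gas interaction stage for the sports car.
; The first MeshComp overlap sets IsSwiched, then loops over every BP_Gas to enable its interact outline.
; Inside that loop it also clears its own outline flag and shows the SportsCar_Pawn Widget component.
; Once switched, Tick calls MoveComponentTo every frame to slide Plane to a fixed relative offset.
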(event `self.meshComp.OnComponentBeginOverlap`
  (params (OverlappedComponent :type "PrimitiveComponent Object Reference") (OtherActor :type "Actor Object Reference") (OtherComp :type "PrimitiveComponent Object Reference") (OtherBodyIndex :type Integer) (bFromSweep :type Boolean) (SweepResult :type "HitResult Structure (by ref)"))
  (if (not (`self.bIsSwiched`))
    (set `self.bIsSwiched` true)
    (bind _outactors (`GameplayStatics.GetAllActorsOfClass` "/Game/Dev/CSK/BP_Gas.BP_Gas_C"))
    (for _array_element _outactors
      (set `InteractionBase.bIsInteractOutlineVisible` true _array_element)
      (set `self.bIsInteractOutlineVisible` false)
      (bind _returnvalue (`GameplayStatics.GetActorOfClass` "/Game/Art/Car/VehicleTemplate/Blueprints/SportsCar/SportsCar_Pawn.SportsCar_Pawn_C"))
      (`SceneComponent.SetVisibility` (`/Game/Art/Car/VehicleTemplate/Blueprints/SportsCar/SportsCar_Pawn.Widget` _returnvalue) true false))))

(event `self.ReceiveTick`
  (params (DeltaSeconds :type "Float (single-precision)"))
  (if (`self.bIsSwiched`)
    (`KismetSystemLibrary.MoveComponentTo` (`self.Plane`) (0.0 -300.0 -1200.0) (struct) false false 2.0)))

(fn `UserConstructionScript`)