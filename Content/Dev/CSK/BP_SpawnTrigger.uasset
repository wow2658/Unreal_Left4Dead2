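; One-shot trigger actor that activates a set of spawners when BP_Hank enters its collision component.
; On the first overlap it sets an IsSpawn guard and calls OnSpawn on every valid entry in the TriggerSpawner array.
; It then destroys every actor in the Actors array and finally destroys itself.
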(event `self.CollComp.OnComponentBeginOverlap`
  (params (OverlappedComponent :type "PrimitiveComponent Object Reference") (OtherActor :type "Actor Object Reference") (OtherComp :type "PrimitiveComponent Object Reference") (OtherBodyIndex :type Integer) (bFromSweep :type Boolean) (SweepResult :type "HitResult Structure (by ref)"))
  (cast `/Game/Dev/LGT/Hank_BP/BP_Hank` OtherActor)
  (if (not (`self.bIsSpawn`))
    (set `self.bIsSpawn` true)
    (for _array_element (`self.TriggerSpawner`)
      (`/Engine/EditorBlueprintResources/StandardMacros.IsValid` _array_element
        (:`Is Valid`
          (`ZombieSpawner.OnSpawn` _array_element))))
    (for _array_element_2 (`self.Actors`)
      (`self.K2_DestroyActor` _array_element_2))
    (`self.K2_DestroyActor`)))

(fn `UserConstructionScript`)