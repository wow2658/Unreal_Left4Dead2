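; BP_ZombieDummy is an actor that spawns a pile of physics-simulated zombie dummy bodies at its location.
; On BeginPlay it adds MeshCount skeletal mesh components with manual attachment, placed at the root's world location, stacked upward at fixed spacing and rolled sideways.
; Each gets the Ch10 character mesh, blocks all channels except Pawn and simulates physics.
; Tick, overlap and construction logic are empty.
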(event `self.ReceiveBeginPlay`
  (for _index (range (`self.meshCount`))
    (bind _returnvalue (`|AddComponentByClass` "/Script/Engine.SkeletalMeshComponent" true (`KismetMathLibrary.MakeTransform` (+ (`SceneComponent.K2_GetComponentLocation` (`self.DefaultSceneRoot`)) (* (`KismetMathLibrary.Vector_Up`) (* _index 50))) (`KismetMathLibrary.MakeRotator` 90.0))))
    (`SkeletalMeshComponent.SetSkeletalMeshAsset` _returnvalue "/Game/Dev/CSK/Zombie/ZombieBasic/Ch10_nonPBR_UE.Ch10_nonPBR_UE")
    (`PrimitiveComponent.SetCollisionObjectType` _returnvalue "ECC_PhysicsBody")
    (`PrimitiveComponent.SetCollisionEnabled` _returnvalue "QueryAndPhysics")
    (`PrimitiveComponent.SetCollisionResponseToAllChannels` _returnvalue "ECR_Block")
    (`PrimitiveComponent.SetCollisionResponseToChannel` _returnvalue "ECC_Pawn" "ECR_Ignore")
    (`PrimitiveComponent.SetSimulatePhysics` _returnvalue true)
    (`PrimitiveComponent.SetStaticWhenNotMoveable` _returnvalue true)))

(fn `UserConstructionScript`)