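; Zombie character Blueprint that varies each zombie's size and keeps its audio playing while it is alive.
; BeginPlay randomly scales the capsule component, and Tick restarts the audio component at a random volume whenever it stops while CurrentHp is above zero.
; An unconnected, never-executed branch would blend pelvis-down ragdoll physics in for a dead, falling zombie and out otherwise.
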(event `self.ReceiveBeginPlay`
  (`SceneComponent.SetRelativeScale3D` (`self.CapsuleComponent`) (`KismetMathLibrary.Conv_DoubleToVector` (`KismetMathLibrary.RandomFloatInRange` 0.9 1.2))))

(event `self.ReceiveTick`
  (params (DeltaSeconds :type "Float (single-precision)"))
  (bind _audiocomp (`self.audioComp`))
  (`|ExecutionSequence`
    (:`then_0`
      (if (> (`self.currentHp`) 0.0)
        (if (not (`AudioComponent.IsPlaying` (`self.audioComp`)))
          (`AudioComponent.SetVolumeMultiplier` _audiocomp (`KismetMathLibrary.RandomFloat`))
          (`AudioComponent.Play` _audiocomp 0.0))))))

(fn `UserConstructionScript`)