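; BP_ZombieGirl is a zombie girl character Blueprint that adds per-instance variation and looping audio.
; On BeginPlay it randomly scales the capsule and briefly randomizes the mesh play rate before restoring normal speed, which staggers animation phase between instances.
; While CurrentHp stays above zero, Tick restarts the audio component at a random volume whenever it stops playing.
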(event `self.ReceiveBeginPlay`
  (bind _mesh (`self.Mesh`))
  (`SceneComponent.SetRelativeScale3D` (`self.CapsuleComponent`) (`KismetMathLibrary.Conv_DoubleToVector` (`KismetMathLibrary.RandomFloatInRange` 0.9 1.2)))
  (`SkeletalMeshComponent.SetPlayRate` _mesh (`KismetMathLibrary.RandomFloatInRange` 0.1 10.0))
  (`KismetSystemLibrary.Delay` 0.2)
  (`SkeletalMeshComponent.SetPlayRate` _mesh 1.0))

(event `self.ReceiveTick`
  (params (DeltaSeconds :type "Float (single-precision)"))
  (bind _audiocomp (`self.audioComp`))
  (if (> (`self.currentHp`) 0.0)
    (if (not (`AudioComponent.IsPlaying` (`self.audioComp`)))
      (`AudioComponent.SetVolumeMultiplier` _audiocomp (`KismetMathLibrary.RandomFloat`))
      (`AudioComponent.Play` _audiocomp 0.0))))

(fn `UserConstructionScript`)