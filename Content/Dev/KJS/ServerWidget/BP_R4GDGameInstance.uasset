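; Game instance Blueprint that tracks players by net ID and assigns each a character index.
; Adding a player reserves the first unused index from 0 to 8 in SelectedCharIndex, but CharactorIndexList records the array position returned by Add.
; Removal treats that recorded number as the value to free, then drops the player's entries from both parallel lists.
; The PlayerList replication callback is empty.
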(event `AddChildPlayerList`
  (params (NetID :type "UniqueNetIdRepl Structure"))
  (bind _selectedcharindex (`self.SelectedCharIndex`))
  (`KismetArrayLibrary.Array_Add` (`self.PlayerList`) NetID)
  (for _index (range 9)
    (if (not (`KismetArrayLibrary.Array_Contains` _selectedcharindex _index))
      (bind _returnvalue (`KismetArrayLibrary.Array_Add` _selectedcharindex _index))
      (break)))
  (`KismetArrayLibrary.Array_Add` (`self.CharactorIndexList`) _returnvalue))

(event `DelChildPlayerList`
  (params (NetID :type "UniqueNetIdRepl Structure"))
  (bind _playerlist (`self.PlayerList`))
  (bind _charactorindexlist (`self.CharactorIndexList`))
  (bind _selectedcharindex (`self.SelectedCharIndex`))
  (bind _returnvalue (`KismetArrayLibrary.Array_Find` _playerlist NetID))
  (bind _returnvalue_2 (`KismetArrayLibrary.Array_Find` _selectedcharindex (`|GetArrayItem` _charactorindexlist _returnvalue)))
  (if (not (< _returnvalue_2 0))
    (`KismetArrayLibrary.Array_Remove` _selectedcharindex _returnvalue_2))
  (`KismetArrayLibrary.Array_Remove` _charactorindexlist _returnvalue)
  (`KismetArrayLibrary.Array_Remove` _playerlist _returnvalue))

(fn `OnRep_PlayerList`)