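; BP_StartDoor is an interactable door that plays a short sequence of Coach and Nick voice lines after BeginPlay.
; Interaction from a LeftCharacter toggles OpenDoor and calls server-named open or close events, with the GameState set as owner.
; These play door sounds and run the DoorRotation timeline forward or in reverse to drive SMDoor's yaw.
; The first timeline completion triggers a one-time Nick "this way" line.
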(event `self.ReceiveBeginPlay`
  (`self.SetOwner` (`GameplayStatics.GetGameState`))
  (`KismetSystemLibrary.Delay` 5.0)
  (`GameplayStatics.PlaySound2D` "/Game/Dev/LGT/Audio/couch/Coach_Join_a.Coach_Join_a" 1.0 1.0 0.0 null null)
  (`KismetSystemLibrary.Delay` 2.0)
  (`GameplayStatics.PlaySound2D` "/Game/Dev/LGT/Audio/nick/Nick_Ready_b.Nick_Ready_b" 1.0 1.0 0.0 null null)
  (`KismetSystemLibrary.Delay` 3.0)
  (`GameplayStatics.PlaySound2D` "/Game/Dev/LGT/Audio/couch/Coach_positive_c.Coach_positive_c" 1.0 1.0 0.0 null null))

(event `/Game/Dev/LGT/Interacted.Interacted`
  (params (Interactor :type "Pawn Object Reference"))
  (cast `LeftCharacter` Interactor)
  (if (`self.OpenDoor`)
    (set `self.OpenDoor` false)
    (`self.ServerCloseDoor`)
    (else
      (set `self.OpenDoor` true)
      (`self.serverOpenDoor`))))

(event `serverOpenDoor`
  (`GameplayStatics.PlaySound2D` "/Game/Dev/LGT/Audio/door_metal_large_open1.door_metal_large_open1" 1.0 1.0 0.0 null null)
  (bind (_direction _dooropen) (`Timeline|DoorRotation` :!label _label)
    (:`Update`
      (`SceneComponent.K2_SetRelativeRotation` (`self.SM_door`) (`KismetMathLibrary.MakeRotator` 0.0 0.0 _dooropen) false false))
    (:`Finished`
      (`/Engine/EditorBlueprintResources/StandardMacros.DoOnce` false
        (:`Completed`
          (`GameplayStatics.PlaySound2D` "/Game/Dev/LGT/Audio/nick/Nick_OkayThisWay_d.Nick_OkayThisWay_d" 1.0 1.0 0.0 null null))))))

(event `ServerCloseDoor`
  (`GameplayStatics.PlaySound2D` "/Game/Dev/LGT/Audio/door_metal_large_close2.door_metal_large_close2" 1.0 1.0 0.0 null null)
  (goto _label :!via `Reverse`))

(fn `UserConstructionScript`)